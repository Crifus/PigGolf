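; BP_PigMode, apparently a game mode, owns the power meter HUD for a cannon shooting game with shots and par.
; On BeginPlay it creates the WBP_PowerMeter widget, stores it as HudRef and adds it to the viewport.
; Custom events relay the current bullet, cannon, shot count and par into that widget, so callers update the HUD through this Blueprint.
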(event EventBeginPlay
  (bind _returnvalue (UserInterface|CreateWidget "/Game/Blueprints/WBP_PowerMeter.WBP_PowerMeter_C"))
  (bind _output_get (Variables|Default|SetHudRef _returnvalue))
  (UserInterface|Viewport|AddtoViewport _output_get 0))

(event EventTick
  (params (DeltaSeconds :type Float%20%28single-precision%29)))

(event EventSetBulletonHUD
  (params (MB :type Pig%20Pawn%20Object%20Reference))
  (Variables|/Game/Blueprints/WBP_PowerMeter.WBP_PowerMeter_C|SetMYBullet (Variables|Default|GetHudRef) MB))

(event EventSetShotsonHUD
  (params (NewShots :type Integer) (NewPar :type Integer))
  (bind _hudref (Variables|Default|GetHudRef))
  (Variables|/Game/Blueprints/WBP_PowerMeter.WBP_PowerMeter_C|SetShots _hudref NewShots)
  (Variables|/Game/Blueprints/WBP_PowerMeter.WBP_PowerMeter_C|SetPar _hudref NewPar))

(event EventSetCannononHUD
  (params (MC :type Cannon%20Pawn%20Object%20Reference))
  (Variables|/Game/Blueprints/WBP_PowerMeter.WBP_PowerMeter_C|SetMYCannon (Variables|Default|GetHudRef) MC))

(fn ConstructionScript)