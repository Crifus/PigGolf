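; BP_Tracker is a pooled physics ball actor tied to the player's BP_CannonPawn.
; At BeginPlay it caches a reference to that pawn.
; When the Ball component hits something, the actor hides, disables collision and physics, and moves itself from the pawn's TrackersOut array back to Trackers.
; The actor is recycled rather than destroyed; nothing in this Blueprint launches or reactivates it.
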(event OnComponentHit(Ball)
  (params (HitComponent :type Primitive%20Component%20Object%20Reference) (OtherActor :type Actor%20Object%20Reference) (OtherComp :type Primitive%20Component%20Object%20Reference) (NormalImpulse :type Vector :default "0, 0, 0") (Hit :type Hit%20Result%20Structure%20%28by%20ref%29))
  (bind _self self)
  (bind _porkref (Variables|Default|GetPorkRef))
  (Rendering|SetActorHiddenInGame true)
  (Collision|SetActorEnableCollision false)
  (Physics|SetSimulatePhysics (Variables|Default|GetBall) false)
  (Utilities|Array|RemoveItem (Variables|/Script/PigGolf.CannonPawn|GetTrackersOut _porkref) _self)
  (Utilities|Array|Add (Variables|/Script/PigGolf.CannonPawn|GetTrackers _porkref) _self))

(event EventBeginPlay
  (bind _asbp_cannon_pawn (Utilities|Casting|CastToBP_CannonPawn (Game|Player|GetPlayerPawn 0)))
  (Variables|Default|SetPorkRef _asbp_cannon_pawn))

(event Collision|EventActorBeginOverlap
  (params (OtherActor :type Actor%20Object%20Reference)))

(event EventTick
  (params (DeltaSeconds :type Float%20%28single-precision%29)))

(fn ConstructionScript)